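; Hour-hand actor for an office clock prop that shows the real system time.
; Every tick it reads the current time and sets its relative rotation around the Y axis.
; The angle combines the 12-hour value with a minute-based offset, so the hand moves gradually between hour marks.
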(event `self.ReceiveTick`
  (params (DeltaSeconds :type "Float (single-precision)"))
  (bind _returnvalue (`KismetMathLibrary.Now`))
  (`self.K2_SetActorRelativeRotation` (`KismetMathLibrary.RotatorFromAxisAndAngle` (0.0 1.0 0.0) (+ (* (`KismetMathLibrary.Conv_IntToDouble` (`KismetMathLibrary.GetHour12` _returnvalue)) 30.0) (/ (* (`KismetMathLibrary.Conv_IntToDouble` (`KismetMathLibrary.GetMinute` _returnvalue)) 6.0) 12.0)))))

(fn `UserConstructionScript`)